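; BP_ItemInGame is a world pickup that shows an item's icon as a Paper2D sprite and its name as text.
; BeginPlay fills the sprite and text from CurrentItem, and Tick turns the text to face the player camera.
; When a BP_TopDownCharacter overlaps its sphere, it adds CurrentItem to the top-down controller's Items array and destroys itself.
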(event OnComponentBeginOverlap(Sphere)
  (params (OverlappedComponent :type Primitive%20Component%20Object%20Reference) (OtherActor :type Actor%20Object%20Reference) (OtherComp :type Primitive%20Component%20Object%20Reference) (OtherBodyIndex :type Integer) (bFromSweep :type Boolean) (SweepResult :type Hit%20Result%20Structure%20%28by%20ref%29))
  (Utilities|Casting|CastToBP_TopDownCharacter OtherActor)
  (Utilities|Array|Add (Variables|/Game/TopDown/Blueprints/BP_TopDownController.BP_TopDownController_C|GetItems (CallFunction|GetTopDownController)) (Variables|Default|GetCurrentItem))
  (Actor|DestroyActor))

(event EventBeginPlay
  (Rendering|Components|Sprite|SetSprite (Variables|Default|GetPaperSprite) (Variables|/Game/Blueprints/Data/BP_DA_Item.BP_DA_Item_C|GetIcones (Variables|Default|GetCurrentItem)))
  (Rendering|Components|TextRender|SetText (Variables|Default|GetTextRender) (Variables|/Game/Blueprints/Data/BP_DA_Item.BP_DA_Item_C|GetName (Variables|Default|GetCurrentItem))))

(event EventTick
  (params (DeltaSeconds :type Float%20%28single-precision%29))
  (Transformation|SetWorldRotation (Variables|Default|GetTextRender) (Math|Rotator|FindLookatRotation (Transformation|GetWorldLocation (Variables|Default|GetTextRender)) (Camera|GetCameraLocation (Variables|/Script/Engine.PlayerController|GetPlayerCameraManager (CallFunction|GetTopDownController)))) false false))

(fn ConstructionScript)